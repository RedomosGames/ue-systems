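; BPC_DamageSystem is a health component that resolves incoming damage and healing for its owner.
; A macro sorts each hit into blocked, damaged or ignored from the dead, invincible and blocking states plus the DamageInfo flags.
; Damage lowers health and fires death or, when interruptible or forced, a damage-response event, while blocks report whether they can be parried.
; Healing clamps health to the maximum and is skipped when dead.
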(fn `F_Heal`
  (params (Amount :type "Float (double-precision)"))
  (returns (NewHealth :type "Float (double-precision)"))
  (if (not (`self.IsDead?`))
    (bind _output_get (set `self.Health` (`KismetMathLibrary.FClamp` (+ (`self.Health`) Amount) 0.0 (`self.MaxHealth`))))
    (return _output_get)))

(fn `F_TakeDamage`
  (params (DamageInfo :type "/Game/SimpleDamage/Blueprints/Data/S_DamageInfo Structure") (DamageCauser :type "Actor Object Reference"))
  (returns (`WasDamaged?` :type Boolean))
  (bind (_amount _damagetype _damageresponse _shoulddamageinvincible_ _canbeblocked_ _canbeparried_ _shouldforceinterrupt_) (break `/Game/SimpleDamage/Blueprints/Data/S_DamageInfo` DamageInfo))
  (`self.M_CanBeDamaged` _shoulddamageinvincible_ _canbeblocked_
    (:`BlockDamage`
      (`self.OnBlocked` _canbeparried_)
      (return false))
    (:`DoDamage`
      (if (not (`self.IsDead?`))
        (bind _output_get (set `self.Health` (- (`self.Health`) _amount)))
        (if (<= _output_get 0.0)
          (set `self.IsDead?` true)
          (`self.OnDeath`)
          (elif (or (`self.IsInterruptible?`) _shouldforceinterrupt_)
            (`self.OnDamageResponse` _damageresponse DamageCauser)))
        (return true)))
    (:`NoDamage`
      (return false))))