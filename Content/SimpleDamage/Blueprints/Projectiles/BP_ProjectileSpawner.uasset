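; A projectile spawner actor that periodically fires projectiles.
; On BeginPlay it starts a looping timer that, while spawning is enabled, spawns a random class from its Projectiles list at the Arrow component's transform.
; Each projectile is owned by the spawner and receives a fixed speed and the spawner's homing flag.
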(event `self.ReceiveBeginPlay`
  (`KismetSystemLibrary.K2_SetTimerDelegate` (delegate `SpawnProjectile`) 3.0 true))

(event `SpawnProjectile`
  (if (`self.ShouldSpawn?`)
    (`|SpawnActorFromClass` (`KismetArrayLibrary.Array_Random` (`self.Projectiles`)) (`SceneComponent.K2_GetComponentToWorld` (`self.Arrow`)) "Undefined" "MultiplyWithRoot" self 500.0 0.0 null (`self.IsHoming?`) null)))

(fn `UserConstructionScript`)