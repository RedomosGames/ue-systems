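; Lightning area-of-effect blast that marks a ground strike point, waits, then triggers.
; On BeginPlay it snaps to the floor under AttackTarget via a visibility trace, whose end multiplies the target's Z by -1000 rather than subtracting an offset.
; It spawns a thunder-strike warning decal there, waits DelayBefore, calls the trigger event, then removes the decal.
; The trigger's effect is not defined in this graph.
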(event `self.ReceiveBeginPlay`
  (`parent.ReceiveBeginPlay`)
  (`self.CE_MoveToFloor`)
  (bind _returnvalue (`GameplayStatics.SpawnDecalAtLocation` "/Game/SimpleDamage/Textures/M_ThunderStrike.M_ThunderStrike" (25.0 256.0 256.0) (`self.K2_GetActorLocation`)))
  (`KismetSystemLibrary.Delay` (`self.DelayBefore`))
  (`self.CE_Trigger`)
  (`/Engine/EditorBlueprintResources/StandardMacros.IsValid` _returnvalue
    (:`Is Valid`
      (`ActorComponent.K2_DestroyComponent` _returnvalue))))

(event `CE_MoveToFloor`
  (bind _attacktarget (`self.AttackTarget`)
    (:`then`
      (bind _returnvalue (`self.K2_GetActorLocation` _attacktarget))
      (bind (_outhit _returnvalue_2) (`KismetSystemLibrary.LineTraceSingle` _returnvalue (* _returnvalue (1.0 1.0 -1000.0)) "TraceTypeQuery1" false (`|MakeArray` _attacktarget)))
      (if _returnvalue_2
        (`self.K2_SetActorLocation` (`.Location` (`GameplayStatics.BreakHitResult` _outhit)))))
    (:`else`)))

(fn `UserConstructionScript`
  (`parent.UserConstructionScript`))