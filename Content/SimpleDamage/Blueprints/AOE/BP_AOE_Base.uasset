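; BP_AOE_Base is a base area-of-effect actor that finds pawns within a radius of its location.
; It triggers through CE_Trigger, optionally one tick after BeginPlay, then runs a sphere overlap that can ignore the instigator.
; Each hit actor is passed to OnAOEOverlapActor and its name is printed, leaving the effect itself outside this graph.
; An optional debug sphere shows the area.
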(event `self.ReceiveBeginPlay`
  ;[1 1 0 0.5] If boolean is True, Trigger on BeginPlay
  (if (`self.TriggerOnBeginPlay`)
    (`KismetSystemLibrary.DelayUntilNextTick`)
    (`self.CE_Trigger`)))

(event `CE_Trigger`
  ;[1 1 0 0.5] Calls AOE Spawn
  (`self.CE_SpawnAOESphere`))

(event `CE_SpawnAOESphere`
  ;[1 1 0 0.5] Creates spehre trace where AOE Spawns / Also creates debug Sphere
  (if (`self.DrawDebugSphere?`)
    (`KismetSystemLibrary.DrawDebugSphere` (`self.K2_GetActorLocation`) (`self.Radius`) 12 (struct :`R` 0.855376 :`G` 0.148631 :`B` 1.0 :`A` 1.0) 2.0 1.0))
  (bind _outactors (`KismetSystemLibrary.SphereOverlapActors` (`self.K2_GetActorLocation`) (`self.Radius`) (`|MakeArray` "ObjectTypeQuery3" :!type "EObjectTypeQuery Enum") null (`|MakeArray` (select `bool` (`self.IgnoreInstigator?`) :`true` (`self.GetInstigator`)) :!type "Actor Object Reference")))
  (for _array_element _outactors
    (`self.OnAOEOverlapActor` _array_element)
    (`KismetSystemLibrary.PrintString` (`KismetSystemLibrary.GetDisplayName` _array_element))))

(fn `UserConstructionScript`)