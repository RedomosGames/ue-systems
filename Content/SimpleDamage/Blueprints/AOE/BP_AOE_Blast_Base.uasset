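; Base Blueprint for area-of-effect blasts in the SimpleDamage system, adding visuals, sound and self-cleanup to the parent's trigger behavior.
; On trigger, it calls the parent logic, attaches the blast particle effect to its root and plays the blast sound at its location.
; The actor destroys itself when the particle system finishes, or after a short delay if no effect is set.
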(event `self.CE_Trigger`
  (`parent.CE_Trigger`)
  (`self.CE_SpawnBlastEffect`)
  (`self.CE_PlayBlastSound`))

(event `CE_PlayBlastSound`
  (bind _blastsound (`self.BlastSound`)
    (:`then`
      (`GameplayStatics.PlaySoundAtLocation` _blastsound (`self.K2_GetActorLocation`) (struct) 1.0 1.0 0.0 null null null null))
    (:`else`)))

(event `CE_SpawnBlastEffect`
  (bind _blasteffect (`self.BlastEffect`)
    (:`then`
      (bind _returnvalue (`GameplayStatics.SpawnEmitterAttached` _blasteffect (`self.RootComponent`)))
      (add `ParticleSystemComponent.OnSystemFinished` _returnvalue (delegate `SystemFinished`)))
    (:`else`
      (`KismetSystemLibrary.Delay` 1.0)
      (`self.K2_DestroyActor`))))

(event `SystemFinished`
  (params (PSystem :type "ParticleSystemComponent Object Reference"))
  (`self.K2_DestroyActor`))

(fn `UserConstructionScript`
  (`parent.UserConstructionScript`))