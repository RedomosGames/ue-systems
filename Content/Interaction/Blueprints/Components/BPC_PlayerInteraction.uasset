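; Player interaction component for a Character that lets it use nearby BPI_Interactable actors via Enhanced Input.
; Capsule overlaps maintain an in-range list, whose first entry gets a screen-space prompt widget created at runtime.
; Each interactable's type selects Press, Hold or Tap logic, with hold time or tap count driving widget progress.
; Interaction fires directly or, optionally, from a montage's "Interact" notify after turning the character toward the target.
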(event `self.ReceiveBeginPlay`
  ;[1 1 0 0.5] On Begin / Get Character Ref
  (bind _ascharacter (cast `Character` (`self.GetOwner`)))
  (bind _output_get (set `self.CharacterRef` _ascharacter))
  (bind _capsulecomponent (`Character.CapsuleComponent` _output_get))
  ;[1 1 0 0.5] Bind to Overlap Events
  (add `PrimitiveComponent.OnComponentBeginOverlap` _capsulecomponent (`|CreateDelegate` :!event `CE_HandleCapsuleOverlapBegin`))
  (add `PrimitiveComponent.OnComponentEndOverlap` _capsulecomponent (`|CreateDelegate` :!event `CE_HandleCapsuleOverlapEnd`))
  ;[1 1 0 0.5] Set Widget Settings and get Ref
  (bind _returnvalue (`|AddComponentByClass` :`self` (`self.GetOwner`) :`Class` "/Script/UMG.WidgetComponent" :`bManualAttachment` true))
  (`WidgetComponent.SetWidgetSpace` _returnvalue "Screen")
  (`WidgetComponent.SetDrawSize` _returnvalue (250.0 30.0))
  (set `self.InteractionComponentRef` _returnvalue))

(event `CE_HandleCapsuleOverlapBegin`
  (params (OverlappedComponent :type "PrimitiveComponent Object Reference") (OtherActor :type "Actor Object Reference") (OtherComp :type "PrimitiveComponent Object Reference") (OtherBodyIndex :type Integer) (bFromSweep :type Boolean) (SweepResult :type "HitResult Structure (by ref)"))
  ;[1 1 0 0.5] Add Interactable In Range
  (if (`KismetSystemLibrary.DoesImplementInterface` OtherActor "/Game/Interaction/Blueprints/Interfaces/BPI_Interactable.BPI_Interactable_C")
    (`KismetArrayLibrary.Array_AddUnique` (`self.InteractablesInRange`) OtherActor)
    (`self.F_RenderInteractionWidget`)))

(event `CE_HandleCapsuleOverlapEnd`
  (params (OverlappedComponent :type "PrimitiveComponent Object Reference") (OtherActor :type "Actor Object Reference") (OtherComp :type "PrimitiveComponent Object Reference") (OtherBodyIndex :type Integer))
  ;[1 1 0 0.5] Remove Interactable Out of Range
  (if (`KismetSystemLibrary.DoesImplementInterface` OtherActor "/Game/Interaction/Blueprints/Interfaces/BPI_Interactable.BPI_Interactable_C")
    (if (== OtherActor (`self.F_GetActiveInteractable`))
      (`self.F_ResetInteractionState`))
    (`KismetArrayLibrary.Array_RemoveItem` (`self.InteractablesInRange`) OtherActor)
    (`self.F_RenderInteractionWidget`)))

(event `EnhancedInput|/Game/Input/Actions/IA_Interact`
  (params (ActionValue :type Boolean) (ElapsedSeconds :type "Float (double-precision)") (TriggeredSeconds :type "Float (double-precision)") (InputAction :type "InputAction Object Reference" :default "/Game/Input/Actions/IA_Interact.IA_Interact"))
  ;[1 1 0 0.5] Enhanced Input
  (:`Started`
    (`self.CE_InteractBegin`))
  (:`Ongoing`
    (`self.OnInteractionPressOnGoing` ElapsedSeconds))
  (:`Completed`
    (clear `self.OnInteractionPressOnGoing`)
    (`self.OnInteractionEnded`)))

(event `CE_InteractBegin`
  (bind _active_interactable (`self.F_GetActiveInteractable`))
  ;[1 1 0 0.5] CE_InteractBegin / Determine interact type
  (`/Engine/EditorBlueprintResources/StandardMacros.IsValid` _active_interactable
    (:`Is Valid`
      (bind _type (message `/Game/Interaction/Blueprints/Interfaces/BPI_Interactable.IF_GetInteractionType` _active_interactable))
      (switch `/Game/Interaction/Blueprints/Data/E_InteractionType` _type
        (:`NewEnumerator0`
          (`KismetSystemLibrary.PrintString` "Interaction Type Not Set"))
        (:`NewEnumerator1`
          (`self.CE_InteractWithActiveInteractable`))
        (:`NewEnumerator2`
          (add `self.OnInteractionPressOnGoing` (`|CreateDelegate` :!event `CE_InteractionHoldOnGoing`))
          (add `self.OnInteractionEnded` (delegate `ResetWidgetProgress`)))
        (:`NewEnumerator3`
          (`self.CE_InteractionTap`))))))

(event `ResetWidgetProgress`
  ;[1 1 0 0.5] CE_InteractBegin / Determine interact type
  (bind _interactionwidgetref (`self.InteractionWidgetRef`)
    (:`then`
      (`/Game/Interaction/Blueprints/Widgets/WBP_InteractionWidget.F_SetProgressPercent` _interactionwidgetref 0.0)
      (remove `self.OnInteractionEnded` (delegate `ResetWidgetProgress`)))
    (:`else`)))

(event `CE_InteractionTap`
  ;[1 1 0 0.5] CE_InteractionTap / Tap Logic
  (`GameplayStatics.PlaySound2D` "/Engine/VREditor/Sounds/UI/Gizmo_Handle_Clicked.Gizmo_Handle_Clicked" 1.0 1.0 0.0 null null)
  (`/Engine/EditorBlueprintResources/StandardMacros.IncrementInt` (`self.CurrentTapCount`)
    (:`  `
      (bind _tapcount (message `/Game/Interaction/Blueprints/Interfaces/BPI_Interactable.IF_GetTapCount` (`self.F_GetActiveInteractable`)))
      (if (<= _tapcount 0)
        (`self.CE_InteractWithActiveInteractable`)
        (else
          (bind _interactionwidgetref (`self.InteractionWidgetRef`)
            (:`then`
              (`/Game/Interaction/Blueprints/Widgets/WBP_InteractionWidget.F_SetProgressPercent` _interactionwidgetref (/ (`self.CurrentTapCount`) _tapcount))
              (if (>= (`self.CurrentTapCount`) _tapcount)
                (`self.CE_InteractWithActiveInteractable`)))
            (:`else`)))))))

(event `CE_InteractionHoldOnGoing` :!signature `self.OnInteractionPressOnGoing`
  (params (ElapsedSeconds :type "Float (double-precision)"))
  (bind _active_interactable (`self.F_GetActiveInteractable`))
  ;[1 1 0 0.5] CE_InteractionHoldOnGoing / Hold Logic
  (`/Engine/EditorBlueprintResources/StandardMacros.IsValid` _active_interactable
    (:`Is Valid`
      (bind _duration (message `/Game/Interaction/Blueprints/Interfaces/BPI_Interactable.IF_GetHoldDuration` _active_interactable))
      (bind _interactionwidgetref (`self.InteractionWidgetRef`)
        (:`then`
          (`/Game/Interaction/Blueprints/Widgets/WBP_InteractionWidget.F_SetProgressPercent` _interactionwidgetref (/ ElapsedSeconds _duration)))
        (:`else`
          _))
      (if (> ElapsedSeconds _duration)
        (`self.CE_InteractWithActiveInteractable`)
        (remove `self.OnInteractionPressOnGoing` (delegate `CE_InteractionHoldOnGoing`))))))

(event `CE_InteractWithActiveInteractable`
  (bind (_returnvalue_roll _returnvalue_pitch _returnvalue_yaw) (`KismetMathLibrary.BreakRotator` (`KismetMathLibrary.FindLookAtRotation` (`Actor.K2_GetActorLocation` (`self.CharacterRef`)) (`self.F_GetActiveInteractableLocation`))))
  ;[1 1 0 0.5] CE_InteractWithActiveInteractable / Interact with Object
  (`/Engine/EditorBlueprintResources/StandardMacros.IsValid` (`self.F_GetActiveInteractable`)
    (:`Is Valid`
      (if (`self.UseAnimation?`)
        (if (`self.LockMovement?`)
          (set `self.CanMove?` false))
        (`Actor.K2_SetActorRotation` (`self.CharacterRef`) (`KismetMathLibrary.MakeRotator` 0.0 0.0 _returnvalue_yaw) false)
        (bind _notifyname (`|PlayMontage` (`Character.Mesh` (`self.CharacterRef`)) (`self.InteractAnimationMonatge`))
          (:`OnNotifyBegin`
            (if (== _notifyname "Interact")
              (message `/Game/Interaction/Blueprints/Interfaces/BPI_Interactable.IF_Interaction` (`self.F_GetActiveInteractable`) (`self.GetOwner`) :!label _label)
              (`self.F_RenderInteractionWidget`)
              (`self.F_ResetInteractionState`)
              (set `self.CanMove?` true))))
        (else
          (goto _label))))))

(fn `F_GetActiveInteractable`
  (returns (`Active Interactable` :type "Actor Object Reference"))
  (return (`|GetArrayItem` (`self.InteractablesInRange`))))

(fn `F_GetActiveInteractableLocation`
  (returns (Location :type "Vector Structure"))
  (bind _active_interactable (`self.F_GetActiveInteractable`))
  (`/Engine/EditorBlueprintResources/StandardMacros.IsValid` _active_interactable
    (:`Is Valid`
      (bind _location (message `/Game/Interaction/Blueprints/Interfaces/BPI_Interactable.IF_GetInteractionLocation` _active_interactable))
      (return (`KismetMathLibrary.SelectVector` (`Actor.K2_GetActorLocation` _active_interactable) _location (`KismetMathLibrary.Vector_IsZero` _location))))))

(fn `F_RenderInteractionWidget`
  (bind _active_interactable (`self.F_GetActiveInteractable`))
  (bind _interactioncomponentref (`self.InteractionComponentRef`))
  (`/Engine/EditorBlueprintResources/StandardMacros.IsValid` _active_interactable
    (:`Is Valid`
      (bind _type (message `/Game/Interaction/Blueprints/Interfaces/BPI_Interactable.IF_GetInteractionType` _active_interactable))
      (bind _prompt (message `/Game/Interaction/Blueprints/Interfaces/BPI_Interactable.IF_GetInteractionPrompt` _active_interactable))
      (bind _returnvalue (`|CreateWidget` "/Game/Interaction/Blueprints/Widgets/WBP_InteractionWidget.WBP_InteractionWidget_C" null _type _prompt))
      (bind _output_get (set `self.InteractionWidgetRef` _returnvalue))
      (`WidgetComponent.SetWidget` _interactioncomponentref _output_get)
      (`SceneComponent.K2_SetWorldLocation` _interactioncomponentref (`self.F_GetActiveInteractableLocation`) false false))
    (:`Is Not Valid`
      (`WidgetComponent.SetWidget` (`self.InteractionComponentRef`) null))))

(fn `F_ResetInteractionState`
  (remove `self.OnInteractionPressOnGoing` (`|CreateDelegate` :!event `CE_InteractionHoldOnGoing`))
  (set `self.CurrentTapCount` 0))