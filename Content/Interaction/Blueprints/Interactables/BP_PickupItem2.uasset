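; BP_PickupItem2 is an interactable pickup actor that implements interaction interface functions.
; On interaction it prints an "Added to the Inventory" message naming itself and the interactor, plays a click sound at its location, then destroys itself.
; No inventory is actually modified.
; Getters expose its prompt, interaction type, hold duration and tap count from variables, and its interaction location from the Scene component's world position.
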(event `/Game/Interaction/Blueprints/Interfaces/BPI_Interactable.IF_Interaction`
  (params (Interactor :type "Actor Object Reference"))
  ;[1 1 0 0.5] IF_Interact / Print Item Name and destroy
  (`KismetSystemLibrary.PrintString` (`KismetTextLibrary.Conv_TextToString` (`|FormatText` "Added {ItemNamme} to the Inventory of {ActorName} " (`KismetSystemLibrary.GetDisplayName` self) (`KismetSystemLibrary.GetDisplayName` Interactor))) true true (struct :`G` 0.66 :`B` 1.0 :`A` 1.0) 5.0)
  (`GameplayStatics.PlaySoundAtLocation` "/Engine/VREditor/Sounds/VR_click3.VR_click3" (`self.K2_GetActorLocation`) (struct) 1.0 1.0 0.0 null null null null)
  (`self.K2_DestroyActor`))

(fn `IF_GetHoldDuration`
  (returns (Duration :type "Float (double-precision)"))
  (return (`self.Duration`)))

(fn `IF_GetInteractionLocation`
  (returns (Location :type "Vector Structure"))
  (return (`SceneComponent.K2_GetComponentLocation` (`self.Scene`))))

(fn `IF_GetInteractionPrompt`
  (returns (Prompt :type Text))
  (return (`self.Prompt`)))

(fn `IF_GetInteractionType`
  (returns (Type :type "/Game/Interaction/Blueprints/Data/E_InteractionType Enum"))
  (return (`self.Type`)))

(fn `IF_GetTapCount`
  (returns (TapCount :type Integer))
  (return (`self.Tap Count`)))

(fn `UserConstructionScript`)