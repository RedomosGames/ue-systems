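; BP_NPC is an interactable NPC actor that turns to face whoever interacts with it.
; On interaction, it snaps its yaw toward the interactor using a look-at rotation and plays a sound at its location.
; Interaction interface getters expose its prompt, type, hold duration and tap count, plus a Scene component's world position as the interaction location.
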(event `/Game/Interaction/Blueprints/Interfaces/BPI_Interactable.IF_Interaction`
  (params (Interactor :type "Actor Object Reference"))
  (bind (_returnvalue_roll _returnvalue_pitch _returnvalue_yaw) (`KismetMathLibrary.BreakRotator` (`KismetMathLibrary.FindLookAtRotation` (`self.K2_GetActorLocation`) (`self.K2_GetActorLocation` Interactor))))
  ;[1 1 0 0.5] Have NPC Look at Player
  (`self.K2_SetActorRotation` (`KismetMathLibrary.MakeRotator` 0.0 0.0 _returnvalue_yaw))
  (`GameplayStatics.PlaySoundAtLocation` "/Engine/VREditor/Sounds/UI/Object_Snaps_To_Another_Actor.Object_Snaps_To_Another_Actor" (`self.K2_GetActorLocation`) (struct) 1.0 1.0 0.0 null null null null))

(fn `IF_GetHoldDuration`
  (returns (Duration :type "Float (double-precision)"))
  (return (`self.Duration`)))

(fn `IF_GetInteractionLocation`
  (returns (Location :type "Vector Structure"))
  (return (`SceneComponent.K2_GetComponentLocation` (`self.Scene`))))

(fn `IF_GetInteractionPrompt`
  (returns (Prompt :type Text))
  (return (`self.Prompt`)))

(fn `IF_GetInteractionType`
  (returns (Type :type "/Game/Interaction/Blueprints/Data/E_InteractionType Enum"))
  (return (`self.Type`)))

(fn `IF_GetTapCount`
  (returns (TapCount :type Integer))
  (return (`self.Tap Count`)))

(fn `UserConstructionScript`)