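; Interactable door that toggles open and closed through the interaction interface.
; Interacting checks IsOpen and calls an open or close event, which flips the flag, plays a sound and plays or reverses a shared timeline driving the mesh's relative yaw.
; Interface getters expose interaction type, hold duration, tap count, a world location from a scene component, and an open or close prompt based on the current state.
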(event `/Game/Interaction/Blueprints/Interfaces/BPI_Interactable.IF_Interaction`
  (params (Interactor :type "Actor Object Reference"))
  ;[1 1 0 0.5] IF_Interact / Decide to open or close door
  (if (`self.IsOpen?`)
    (`self.CE_CloseDoor`)
    (else
      (`self.CE_OpenDoor`))))

(event `CE_OpenDoor`
  ;[1 1 0 0.5] Door Timeline Animation
  (set `self.IsOpen?` true)
  (`GameplayStatics.PlaySoundAtLocation` "/Engine/VREditor/Sounds/UI/Enter_Simulate.Enter_Simulate" (`self.K2_GetActorLocation`) (struct) 1.0 1.0 0.0 null null null null)
  (bind (_direction _zrotation) (`Timeline|OpenDoorTimeline` :!label _label)
    (:`Update`
      (`SceneComponent.K2_SetRelativeRotation` (`self.StaticMesh`) (`KismetMathLibrary.MakeRotator` 0.0 0.0 _zrotation) false false))))

(event `CE_CloseDoor`
  ;[1 1 0 0.5] Door Timeline Animation
  (set `self.IsOpen?` false)
  (`GameplayStatics.PlaySoundAtLocation` "/Engine/VREditor/Sounds/UI/Leave_Simulate.Leave_Simulate" (`self.K2_GetActorLocation`) (struct) 1.0 1.0 0.0 null null null null)
  (goto _label :!via `Reverse`))

(fn `IF_GetHoldDuration`
  (returns (Duration :type "Float (double-precision)"))
  (return (`self.Duration`)))

(fn `IF_GetInteractionLocation`
  (returns (Location :type "Vector Structure"))
  (return (`SceneComponent.K2_GetComponentLocation` (`self.Scene`))))

(fn `IF_GetInteractionPrompt`
  (returns (Prompt :type Text))
  (return (select `bool` (`self.IsOpen?`) :`false` "to open the door" :`true` "to close the door" :!type "Text")))

(fn `IF_GetInteractionType`
  (returns (Type :type "/Game/Interaction/Blueprints/Data/E_InteractionType Enum"))
  (return (`self.Type`)))

(fn `IF_GetTapCount`
  (returns (TapCount :type Integer))
  (return (`self.Tap Count`)))

(fn `UserConstructionScript`)