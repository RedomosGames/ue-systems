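; Inventory component that stores items and their quantities in a Content map.
; Add, remove and query functions work on that map, with removal deleting entries that reach zero and both changes firing the OnInventoryUpdated dispatcher.
; Pressing the 1 key debug-prints the contents and toggles the WBP_PlayerDisplay widget, creating it for player 0 or removing it.
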(event `Key|One`
  (params (Key :type "Key Structure"))
  ;[1 1 0 0.5] Toggle The Inventory Widget
  (:`Pressed`
    (`self.F_DEBUG_PrintContent`)
    (bind _playerdisplaywidget (`self.PlayerDisplayWidget`)
      (:`then`
        (`Widget.RemoveFromParent` _playerdisplaywidget)
        (set `self.PlayerDisplayWidget` null))
      (:`else`
        (bind _returnvalue (`|CreateWidget` "/Game/SimpleInventory/Blueprints/Widgets/WBP_PlayerDisplay.WBP_PlayerDisplay_C" (`GameplayStatics.GetPlayerController` 0)))
        (bind _output_get (set `self.PlayerDisplayWidget` _returnvalue))
        (`UserWidget.AddToViewport` _output_get 0)))))

(fn `F_AddToInventory`
  (params (Item :type "/Game/SimpleInventory/Blueprints/DataAssets/DA_Base Object Reference") (Quantity :type Integer))
  (`BlueprintMapLibrary.Map_Add` (`self.Content`) Item (+ Quantity (`BlueprintMapLibrary.Map_Find` (`self.Content`) Item)))
  (`self.OnInventoryUpdated`))

(fn `F_DEBUG_PrintContent`
  (bind _content (`self.Content`))
  (bind _keys (`BlueprintMapLibrary.Map_Keys` _content))
  (for (_array_element _array_index) _keys
    (`KismetSystemLibrary.PrintString` (`KismetTextLibrary.Conv_TextToString` (`|FormatText` "{Index} : {Name} = {Quantity}" _array_index (`/Game/SimpleInventory/Blueprints/DataAssets/DA_Base.Name` _array_element) (`BlueprintMapLibrary.Map_Find` _content _array_element))))))

(fn `F_QueryInventory`
  (params (Item :type "/Game/SimpleInventory/Blueprints/DataAssets/DA_Base Object Reference"))
  (returns (Quantity :type Integer))
  (return (`BlueprintMapLibrary.Map_Find` (`self.Content`) Item)))

(fn `F_RemoveFromInventory`
  (params (Item :type "/Game/SimpleInventory/Blueprints/DataAssets/DA_Base Object Reference") (Quantity :type Integer))
  (bind _returnvalue (`KismetMathLibrary.Max` (- (`BlueprintMapLibrary.Map_Find` (`self.Content`) Item) Quantity)))
  (if (== _returnvalue 0)
    (`BlueprintMapLibrary.Map_Remove` (`self.Content`) Item)
    (`self.OnInventoryUpdated`)
    (else
      (`BlueprintMapLibrary.Map_Add` (`self.Content`) Item _returnvalue)
      (`self.OnInventoryUpdated`))))