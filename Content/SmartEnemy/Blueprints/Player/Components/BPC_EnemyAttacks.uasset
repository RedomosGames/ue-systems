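; Attack component that performs magic spell and bullet attacks for its owning actor.
; The spell spawns a projectile with a target that ignores the owner and damages the actor it hits on impact, then broadcasts attack end.
; The bullet is an instant line trace against pawns, with no attack-end broadcast.
; Both deliver damage through an interface message and report a damage event, likely for AI perception.
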(event `CE_MagicSpell`
  (params (SpawnTransform :type "Transform Structure") (Target :type "Actor Object Reference") (DamageInfo :type "/Game/SimpleDamage/Blueprints/Data/S_DamageInfo Structure"))
  (bind _returnvalue (`|SpawnActorFromClass` "/Game/SimpleDamage/Blueprints/Projectiles/BP_Projectile_1.BP_Projectile_1_C" SpawnTransform "Undefined" "MultiplyWithRoot" (`self.GetOwner`) 1000.0 0.0 Target false null))
  (add `/Game/SimpleDamage/Blueprints/Projectiles/BP_Projectile_Base.OnProjectileImpact` _returnvalue (delegate `B_OnProjectileImpact`))
  (`PrimitiveComponent.IgnoreActorWhenMoving` (`/Game/SimpleDamage/Blueprints/Projectiles/BP_Projectile_Base.BoxCollision` _returnvalue) (`self.GetOwner`) true))

(event `B_OnProjectileImpact`
  (params (OtherActor :type "Actor Object Reference") (Hit :type "HitResult Structure"))
  (bind _returnvalue (`self.GetOwner`))
  (message `/Game/SimpleDamage/Blueprints/Interfaces/BPI_Damagable.IF_TakeDamage` OtherActor (stale `CE_MagicSpell` DamageInfo))
  (`AISense_Damage.ReportDamageEvent` OtherActor _returnvalue (`.Amount_2_53500D7C4D64122E874E04B31BC77AE0` (break `/Game/SimpleDamage/Blueprints/Data/S_DamageInfo` (stale `CE_MagicSpell` DamageInfo))) (`Actor.K2_GetActorLocation` _returnvalue))
  (`self.OnAttackEnded`))

(event `CE_FireBullet`
  (params (TraceStart :type "Vector Structure") (TraceEnd :type "Vector Structure") (DamageInfo :type "/Game/SimpleDamage/Blueprints/Data/S_DamageInfo Structure"))
  (bind _returnvalue (`self.GetOwner`))
  (bind (_outhit _returnvalue_2) (`KismetSystemLibrary.LineTraceSingleForObjects` TraceStart TraceEnd (`|MakeArray` "ObjectTypeQuery3" :!type "EObjectTypeQuery Enum")))
  (if _returnvalue_2
    (bind (_bblockinghit _binitialoverlap _time _distance _location _impactpoint _normal _impactnormal _physmat _hitactor) (`GameplayStatics.BreakHitResult` _outhit))
    (message `/Game/SimpleDamage/Blueprints/Interfaces/BPI_Damagable.IF_TakeDamage` _hitactor DamageInfo)
    (`AISense_Damage.ReportDamageEvent` _hitactor _returnvalue (`.Amount_2_53500D7C4D64122E874E04B31BC77AE0` (break `/Game/SimpleDamage/Blueprints/Data/S_DamageInfo` DamageInfo)) (`Actor.K2_GetActorLocation` _returnvalue))))