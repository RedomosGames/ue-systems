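; BP_Enemy_Ranged is the rifle-wielding enemy Blueprint, extending a parent enemy's BeginPlay with immediate weapon equipping.
; Equipping spawns BP_Weapon_Rifle, attaches it to the hand socket and signals that it is equipped.
; Attacking plays a fire montage whose notify traces visibility from weapon to the AI controller's attack target.
; An unobstructed trace sends fixed damage through an interface, and montage completion or interruption signals attack end.
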(event `self.ReceiveBeginPlay`
  (`parent.ReceiveBeginPlay`)
  (`self.IF_EquipWeapon`))

(event `/Game/SmartEnemy/Blueprints/Enemies/AI/BPI_EnemyAI.IF_EquipWeapon`
  (bind _returnvalue (`|SpawnActorFromClass` "/Game/SmartEnemy/Blueprints/Weapons/BP_Weapon_Rifle.BP_Weapon_Rifle_C" (`KismetMathLibrary.MakeTransform` (0.0 0.0 0.0)) "Undefined" "MultiplyWithRoot" null null))
  (bind _output_get (set `self.WeaponActor` _returnvalue))
  (`self.K2_AttachToComponent` _output_get (`self.Mesh`) "hand_r_rifle_socket" "SnapToTarget" "SnapToTarget" "SnapToTarget" true)
  (set `self.IsWieldingWeapon` true)
  (`self.OnWeaponEquip`))

(event `/Game/SmartEnemy/Blueprints/Enemies/AI/BPI_EnemyAI.IF_Attack`
  (bind _notifyname (`|PlayMontage` (`self.Mesh`) "/Game/SmartEnemy/Animations/RifleFire_Montage.RifleFire_Montage")
    (:`OnCompleted`
      (`self.OnAttackEnd` :!label _label))
    (:`OnInterrupted`
      (goto _label))
    (:`OnNotifyBegin`
      (switch `name` _notifyname
        (:`Fire`
          (bind _asaic_enemy_base (cast `/Game/SmartEnemy/Blueprints/Enemies/AI/AIC_Enemy_Base` (`AIBlueprintHelperLibrary.GetAIController` self)))
          (bind _attacktarget (`/Game/SmartEnemy/Blueprints/Enemies/AI/AIC_Enemy_Base.AttackTarget` _asaic_enemy_base)
            (:`then`
              (bind (_outhit _returnvalue) (`KismetSystemLibrary.LineTraceSingle` :`Start` (`self.K2_GetActorLocation` (`self.WeaponActor`)) :`End` (`self.K2_GetActorLocation` _attacktarget) :`TraceChannel` "TraceTypeQuery1" :`DrawDebugType` "ForDuration"))
              (if (not _returnvalue)
                (message `/Game/SimpleDamage/Blueprints/Interfaces/BPI_Damagable.IF_TakeDamage` _attacktarget (make `/Game/SimpleDamage/Blueprints/Data/S_DamageInfo` 20.0 "NewEnumerator2"))))
            (:`else`)))))))

(fn `UserConstructionScript`
  (`parent.UserConstructionScript`))