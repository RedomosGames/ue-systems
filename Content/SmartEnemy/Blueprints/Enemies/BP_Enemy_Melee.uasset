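; Melee enemy child Blueprint that implements sword equip and unequip, attacking and blocking through interface and custom events.
; Montage notifies time the sword's spawn, socket attach and destruction, plus a forward sphere trace that deals attack damage.
; The damage system component is uninterruptible during attacks and tracks blocking; blocked hits play a reaction montage before ending the block.
; Dispatchers report when attack, equip, unequip and block finish.
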(event `self.ReceiveBeginPlay`
  (`parent.ReceiveBeginPlay`))

(event `/Game/SmartEnemy/Blueprints/Enemies/AI/BPI_EnemyAI.IF_Attack`
  (bind _returnvalue (`self.K2_GetActorLocation`))
  (bind _notifyname (`|PlayMontage` (`self.Mesh`) "/Game/SmartEnemy/Animations/Attack_Montage.Attack_Montage")
    (:`then`
      (set `/Game/SimpleDamage/Blueprints/Components/BPC_DamageSystem.IsInterruptible?` false (`self.BPC_DamageSystem`)))
    (:`OnCompleted`
      (`self.OnAttackEnd` :!label _label)
      (set `/Game/SimpleDamage/Blueprints/Components/BPC_DamageSystem.IsInterruptible?` true (`self.BPC_DamageSystem`)))
    (:`OnInterrupted`
      (goto _label))
    (:`OnNotifyBegin`
      (switch `name` _notifyname
        (:`Attack`
          (bind (_outhit _returnvalue_2) (`KismetSystemLibrary.SphereTraceSingleForObjects` :`Start` _returnvalue :`End` (+ _returnvalue (* (`self.GetActorForwardVector`) 200.0)) :`Radius` 20.0 :`ObjectTypes` (`|MakeArray` "ObjectTypeQuery3" :!type "EObjectTypeQuery Enum") :`DrawDebugType` "ForDuration"))
          (if _returnvalue_2
            (message `/Game/SimpleDamage/Blueprints/Interfaces/BPI_Damagable.IF_TakeDamage` (`.HitActor` (`GameplayStatics.BreakHitResult` _outhit)) (make `/Game/SimpleDamage/Blueprints/Data/S_DamageInfo` 25.0 "NewEnumerator1") self)))))))

(event `/Game/SmartEnemy/Blueprints/Enemies/AI/BPI_EnemyAI.IF_EquipWeapon`
  (bind _notifyname (`|PlayMontage` (`self.Mesh`) "/Game/SmartEnemy/Animations/Equip_Montage.Equip_Montage")
    (:`OnCompleted`
      (`self.OnWeaponEquip`))
    (:`OnNotifyBegin`
      (switch `name` _notifyname
        (:`Equip`
          (bind _returnvalue (`|SpawnActorFromClass` "/Game/SmartEnemy/Blueprints/Weapons/BP_Weapon_Sword.BP_Weapon_Sword_C" (`self.GetTransform`) "Undefined" "MultiplyWithRoot" null null))
          (bind _output_get (set `self.WeaponActor` _returnvalue))
          (`self.K2_AttachToComponent` _output_get (`self.Mesh`) "hand_r_sword_socket" "SnapToTarget" "SnapToTarget" "SnapToTarget" true)
          (set `self.IsWieldingWeapon` true))))))

(event `/Game/SmartEnemy/Blueprints/Enemies/AI/BPI_EnemyAI.IF_UnequipWeapon`
  (bind _notifyname (`|PlayMontage` (`self.Mesh`) "/Game/SmartEnemy/Animations/Remove_Montage.Remove_Montage")
    (:`OnCompleted`
      (`self.OnWeaponUnequip`))
    (:`OnNotifyBegin`
      (switch `name` _notifyname
        (:`Remove`
          (set `self.IsWieldingWeapon` false)
          (`self.K2_DestroyActor` (`self.WeaponActor`)))))))

(event `CE_StartBlock`
  ;[0 1 0 0.5] Blocking
  (`MovementComponent.StopMovementImmediately` (`self.CharacterMovement`))
  (set `/Game/SimpleDamage/Blueprints/Components/BPC_DamageSystem.IsBlocking?` true (`self.BPC_DamageSystem`))
  (set `self.BlockingState` "NewEnumerator2")
  (`|PlayMontage` (`self.Mesh`) "/Game/SmartEnemy/Animations/BlockMelee_Montage.BlockMelee_Montage"))

(event `self.BPC_DamageSystem.OnBlocked`
  (params (`CanBeParried?` :type Boolean))
  ;[0 1 0 0.5] Blocking
  (set `self.BlockingState` "NewEnumerator3")
  (`|PlayMontage` (`self.Mesh`) "/Game/SmartEnemy/Animations/BlockHit_Montage.BlockHit_Montage"
    (:`OnCompleted`
      (`self.CE_EndBlock` :!label _label_2))
    (:`OnInterrupted`
      (if (`|EnumInequality` (`self.BlockingState`) "NewEnumerator3")
        (goto _label_2)))))

(event `CE_EndBlock`
  ;[0 1 0 0.5] Blocking
  (set `/Game/SimpleDamage/Blueprints/Components/BPC_DamageSystem.IsBlocking?` false (`self.BPC_DamageSystem`))
  (set `self.BlockingState` "NewEnumerator1")
  (`self.OnBlockEnded`))

(fn `UserConstructionScript`
  (`parent.UserConstructionScript`))