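; BPC_SmartGrid is a Blueprint component that snaps locations to a uniform square grid.
; Its grid-location function rounds X and Y to the nearest cell center, using GridSize for cell spacing and GridOffset to shift the grid origin.
; The input height is discarded, so the result always sits at the Z of GridOffset.
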(fn `F_GetGridLocation`
  (params (Location :type "Vector Structure"))
  (returns (LocationOnGrid :type "Vector Structure"))
  (bind _gridsize (`self.GridSize`))
  (bind _gridsize_2 (`self.GridSize`))
  (bind (_gridoffset_x _gridoffset_y) (`KismetMathLibrary.BreakVector` (`self.GridOffset`)))
  (bind _returnvalue (/ (`self.GridSize`) 2.0))
  (bind _returnvalue_2 (/ (`self.GridSize`) 2.0))
  (return (+ (`KismetMathLibrary.MakeVector` (+ (* (`KismetMathLibrary.Conv_IntToDouble` (`KismetMathLibrary.Round` (/ (- (- Location_X _returnvalue) _gridoffset_x) _gridsize))) _gridsize_2) _returnvalue_2) (+ (* (`KismetMathLibrary.Conv_IntToDouble` (`KismetMathLibrary.Round` (/ (- (- Location_Y _returnvalue) _gridoffset_y) _gridsize))) _gridsize_2) _returnvalue_2)) (`self.GridOffset`))))